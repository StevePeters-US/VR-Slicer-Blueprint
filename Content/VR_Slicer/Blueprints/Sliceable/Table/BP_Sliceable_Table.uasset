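; Sliceable table assembled from child actors for the top, skirts and legs, held together by breakable physics.
; On BeginPlay it spawns physics constraints between the pieces' procedural meshes, joining top to skirts and legs, and each leg to its adjacent skirts.
; Joints lock all axes and disable collision between joined parts, breaking only under linear force.
; It also copies its slice impulse threshold to every BP_Sliceable child.
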(event EventBeginPlay
  (Utilities|FlowControl|Sequence
    (:then_0
      (CallFunction|AddPhysicsConstraint (Variables|Default|GetBP_Table_Top) (Variables|Default|GetBP_Table_Skirt_Front))
      (CallFunction|AddPhysicsConstraint (Variables|Default|GetBP_Table_Top) (Variables|Default|GetBP_Table_Skirt_Back))
      (CallFunction|AddPhysicsConstraint (Variables|Default|GetBP_Table_Top) (Variables|Default|GetBP_Table_Skirt_Left))
      (CallFunction|AddPhysicsConstraint (Variables|Default|GetBP_Table_Top) (Variables|Default|GetBP_Table_Skirt_Right)))
    (:then_1
      (CallFunction|AddPhysicsConstraint (Variables|Default|GetBP_Table_Top) (Variables|Default|GetBP_Table_Leg_1))
      (CallFunction|AddPhysicsConstraint (Variables|Default|GetBP_Table_Top) (Variables|Default|GetBP_Table_Leg_2))
      (CallFunction|AddPhysicsConstraint (Variables|Default|GetBP_Table_Top) (Variables|Default|GetBP_Table_Leg_3))
      (CallFunction|AddPhysicsConstraint (Variables|Default|GetBP_Table_Top) (Variables|Default|GetBP_Table_Leg_4)))
    (:then_2
      (CallFunction|AddPhysicsConstraint (Variables|Default|GetBP_Table_Leg_1) (Variables|Default|GetBP_Table_Skirt_Front))
      (CallFunction|AddPhysicsConstraint (Variables|Default|GetBP_Table_Leg_1) (Variables|Default|GetBP_Table_Skirt_Right))
      (CallFunction|AddPhysicsConstraint (Variables|Default|GetBP_Table_Leg_2) (Variables|Default|GetBP_Table_Skirt_Front))
      (CallFunction|AddPhysicsConstraint (Variables|Default|GetBP_Table_Leg_2) (Variables|Default|GetBP_Table_Skirt_Left)))
    (:then_3
      (CallFunction|AddPhysicsConstraint (Variables|Default|GetBP_Table_Leg_3) (Variables|Default|GetBP_Table_Skirt_Left))
      (CallFunction|AddPhysicsConstraint (Variables|Default|GetBP_Table_Leg_3) (Variables|Default|GetBP_Table_Skirt_Back))
      (CallFunction|AddPhysicsConstraint (Variables|Default|GetBP_Table_Leg_4) (Variables|Default|GetBP_Table_Skirt_Back))
      (CallFunction|AddPhysicsConstraint (Variables|Default|GetBP_Table_Leg_4) (Variables|Default|GetBP_Table_Skirt_Right)))
    (:then_4
      (for _array_element (Actor|GetAllChildActors true)
        (bind _asbp_sliceable (Utilities|Casting|CastToBP_Sliceable _array_element))
        (Variables|/Game/VR_Slicer/Blueprints/Sliceable/BP_Sliceable.BP_Sliceable_C|SetSliceImpulseThreshold _asbp_sliceable (Variables|Default|GetSliceImpuleThreshold))))))

(event Collision|EventActorBeginOverlap
  (params (OtherActor :type Actor%20Object%20Reference)))

(event EventTick
  (params (DeltaSeconds :type Float%20%28single-precision%29)))

(fn ConstructionScript)

(fn AddPhysicsConstraint
  (params (self2 :type Child%20Actor%20Component%20Object%20Reference) (self3 :type Child%20Actor%20Component%20Object%20Reference))
  (bind _returnvalue (AddComponent|AddPhysicsConstraintComponent false))
  (bind _output_get (LocalVariables|SetPhysicsConstraint _returnvalue))
  (bind _proceduralmesh (Utilities|GetChildProcMesh self2))
  (bind _proceduralmesh_2 (Utilities|GetChildProcMesh self3))
  (Class|PhysicsConstraintComponent|SetConstrainedComponents _output_get _proceduralmesh "None" _proceduralmesh_2 "None")
  (Class|PhysicsConstraintComponent|SetLinearBreakable (LocalVariables|GetPhysicsConstraint) true (Variables|Default|GetLinearBreakThreshold))
  (Class|PhysicsConstraintComponent|SetAngularBreakable (LocalVariables|GetPhysicsConstraint) false (Variables|Default|GetAngularBreakThreshold))
  (Class|PhysicsConstraintComponent|SetLinearXLimit (LocalVariables|GetPhysicsConstraint) "LCM_Locked" 0.0)
  (Class|PhysicsConstraintComponent|SetLinearYLimit (LocalVariables|GetPhysicsConstraint) "LCM_Locked" 0.0)
  (Class|PhysicsConstraintComponent|SetLinearZLimit (LocalVariables|GetPhysicsConstraint) "LCM_Locked" 0.0)
  (Class|PhysicsConstraintComponent|SetAngularSwing1Limit (LocalVariables|GetPhysicsConstraint) "ACM_Locked" 0.0)
  (Class|PhysicsConstraintComponent|SetAngularSwing2Limit (LocalVariables|GetPhysicsConstraint) "ACM_Locked" 0.0)
  (Class|PhysicsConstraintComponent|SetAngularTwistLimit (LocalVariables|GetPhysicsConstraint) "ACM_Locked" 0.0)
  (Class|PhysicsConstraintComponent|SetDisableCollision (LocalVariables|GetPhysicsConstraint) true))