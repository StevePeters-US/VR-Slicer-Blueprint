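; BP_Sliceable is a VR Slicer actor that can be cut repeatedly into physics-simulated pieces.
; Construction copies a static mesh into a procedural mesh with exterior materials and stores it as the first chunk.
; SliceMesh starts the actor's lifespan on the first call, then gates cuts on impulse, chunk size and a per-chunk cooldown.
; Each cut caps the interior with its own material and stores the new half with a timestamp.
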(fn ConstructionScript
  (Utilities|Array|Clear (Variables|Default|GetStored%20Procedural%20Mesh%20Chunks))
  (CallFunction|CreateProceduralMeshCopy))

(fn SliceMesh
  (params (NormalImpulse :type Vector) (ProceduralMeshToSlice :type Procedural%20Mesh%20Component%20Object%20Reference) (Hit%20Location :type Vector) (Hit%20Normal :type Vector))
  (Utilities|SetActorLifespanonFirstSlice)
  (Utilities|CheckSliceImpulse NormalImpulse)
  (Utilities|CheckChunkSize ProceduralMeshToSlice)
  (Utilities|CheckChunkSliceTimeM ProceduralMeshToSlice
    (:Can%20Slice
      (bind _outotherhalfprocmesh (Class|KismetProceduralMeshLibrary|SliceProceduralMesh ProceduralMeshToSlice Hit%20Location Hit%20Normal true "CreateNewSectionForCap" (Variables|Setup|GetInteriorMaterial)))
      (Utilities|StoreChunk _outotherhalfprocmesh)
      (Physics|SetSimulatePhysics _outotherhalfprocmesh true)
      (return _outotherhalfprocmesh))))

(fn DestroyChunk
  (params (ProceduralMesh_Chunk :type Procedural%20Mesh%20Component%20Object%20Reference))
  (Components|DestroyComponent ProceduralMesh_Chunk))

(fn CreateProceduralMeshCopy
  (Components|StaticMesh|SetStaticMesh (Variables|Components|GetStaticMesh) (Variables|Setup|GetMeshToCopy))
  (Class|KismetProceduralMeshLibrary|CopyProceduralMeshfromStaticMeshComponent (Variables|Components|GetStaticMesh) 0 (Variables|Components|GetProceduralMesh) true)
  (for (_array_element _array_index) (Variables|Setup|GetExteriorMaterial)
    (Rendering|Material|SetMaterial (Variables|Components|GetProceduralMesh) _array_index _array_element))
  (Utilities|StoreChunk (Variables|Components|GetProceduralMesh))
  (Components|DestroyComponent (Variables|Components|GetStaticMesh)))

(fn CheckChunkSliceTime
  (params (Procedural%20mesh%20chunk :type Procedural%20Mesh%20Component%20Object%20Reference))
  (bind (_array_element _array_index) (Utilities|Array|ForEachLoopwithBreak (Variables|Default|GetStored%20Procedural%20Mesh%20Chunks) :!label _label)
    (:LoopBody
      (if (== (.Proceduralmeshchunk (Utilities|Struct|BreakSliceable_Chunk _array_element)) Procedural%20mesh%20chunk)
        (if (> (Actor|GetGameTimeSinceCreation) (+ (Variables|Setup|GetDelay%20Time) (.TimeAtLastSlice (Utilities|Struct|BreakSliceable_Chunk _array_element))))
          (bind _structout (Utilities|Struct|SetmembersinSliceable_Chunk _array_element (Actor|GetGameTimeSinceCreation)))
          (Utilities|Array|SetArrayElem (Variables|Default|GetStored%20Procedural%20Mesh%20Chunks) _array_index _structout)
          (LocalVariables|SetChunk%20Can%20Slice true)
          (goto _label Break))))
    (:Completed
      (return (LocalVariables|GetChunk%20Can%20Slice)))))