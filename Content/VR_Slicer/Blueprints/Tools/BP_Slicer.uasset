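; BP_Slicer is a VR pickup tool that cuts BP_Sliceable procedural meshes on hit.
; Tick samples tip movement into a fixed-length queue, averaging it into a smoothed swing direction.
; Hit slices along either the cross product of blade and swing directions or a DamageDirection component.
; Impulse can be scaled by a curve evaluated on how squarely child damage-direction arrows oppose the hit normal.
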(event EventTick
  (params (DeltaSeconds :type Float%20%28single-precision%29))
  (bind _tipfollower (Variables|Components|GetTipFollower))
  (bind _returnvalue (Transformation|GetWorldLocation _tipfollower))
  (CallFunction|GetMovementDirection)
  ;[0 1 0.9938] Debug
  (if (Variables|Debug|GetDebugMovementDirection)
    (Rendering|Debug|DrawDebugArrow _returnvalue (+ _returnvalue (* (Math|Vector|Normalize (Variables|Default|GetCurrent_MovementDirection)) 5e+01)) 25.0 "(R=1.000000,G=0.000000,B=0.922276,A=1.000000)" 0.0 1.0)))

(event EventPickup
  (params (AttachTo :type Scene%20Component%20Object%20Reference))
  ;[1 1 1] Required by pickup interface so that VR hands can pick up slicers
  (Physics|SetSimulatePhysics (Variables|Components|GetSlicer_SM) false)
  (Transformation|AttachComponentToComponent (VehicleSound|GetRootComponent) AttachTo "None" "SnapToTarget" "SnapToTarget" "KeepWorld" false)
  (Transformation|AddActorLocalOffset (Variables|Setup|GetGrabLocationOffset) false false)
  (Transformation|AddActorLocalRotation (Variables|Setup|GetGrabRotationOffset) false false))

(event Collision|EventHit
  (params (MyComp :type Primitive%20Component%20Object%20Reference) (Other :type Actor%20Object%20Reference) (OtherComp :type Primitive%20Component%20Object%20Reference) (bSelfMoved :type Boolean) (HitLocation :type Vector :default "0, 0, 0") (HitNormal :type Vector :default "0, 0, 0") (NormalImpulse :type Vector :default "0, 0, 0") (Hit :type Hit%20Result%20Structure%20%28by%20ref%29))
  (bind _asbp_sliceable (Utilities|Casting|CastToBP_Sliceable Other))
  (bind _asprocedural_mesh_component (Utilities|Casting|CastToProceduralMeshComponent OtherComp))
  ;[1 1 1] Get Hit impulse based on direction
  (bind _damage_direction_modifier (CallFunction|CalcDamageDirectionModifier HitNormal))
  (Default|SliceMesh _asbp_sliceable (* (select (Variables|Setup|GetUseDamageDirection%20For%20Impulse) (* NormalImpulse _damage_direction_modifier) NormalImpulse) (Variables|Setup|GetSliceImpulseMultiplier)) _asprocedural_mesh_component (.ImpactPoint (Collision|BreakHitResult Hit)) (select (Variables|Setup|GetUseDamageDirection%20For%20Slicing%20Direction) (Math|Vector|GetRightVector (Variables|Components|GetDamageDirection)) (Math|Vector|CrossProduct (Variables|Default|GetHiltDirection) (Variables|Default|GetCurrent_MovementDirection)))))

(event EventDrop
  ;[1 1 1] Required by pickup interface so that VR hands can pick up slicers
  (Physics|SetSimulatePhysics (Variables|Components|GetSlicer_SM) true)
  (Transformation|DetachFromActor "KeepWorld" "KeepWorld" "KeepWorld"))

(event EventBeginPlay
  (Variables|Default|SetTime%20Between%20Smoothing%20Iteration (/ (Variables|Setup|GetMovementDirectionSmoothingLength) (Math|Conversions|ToFloat(Integer) (Variables|Setup|GetSmoothingTimesteps)))))

(fn ConstructionScript)

(fn GetMovementDirection
  (bind _stored_movementdirections (Variables|Default|GetStored_MovementDirections))
  (bind _returnvalue (Utilities|Array|Length _stored_movementdirections))
  (bind _returnvalue_2 (- _returnvalue 1))
  ;[1 1 1] Should we record another movement timestep?
  (if (> (Actor|GetGameTimeSinceCreation) (+ (Variables|Default|GetTime%20Between%20Smoothing%20Iteration) (LocalVariables|GetPreviousTime)))
    ;[1 1 1] Reset Timer
    (LocalVariables|SetPreviousTime (Actor|GetGameTimeSinceCreation))
    ;[1 1 1] Get Current Movement Direction
    (Variables|Default|SetPrevLoc (Variables|Default|GetCur_Loc))
    (Variables|Default|SetCur_Loc (Transformation|GetWorldLocation (Variables|Components|GetTipFollower)))
    (bind _output_get (LocalVariables|SetAddToStoredMovmentDirections (- (Variables|Default|GetCur_Loc) (Variables|Default|GetPrevLoc))))
    ;[1 1 1] Is Stored Movement Directions Queue filled?
    (if (>= (Utilities|Array|Length (Variables|Default|GetStored_MovementDirections)) (Variables|Setup|GetSmoothingTimesteps))
      ;[1 1 1] Add Movement Direction To Queue
      (for _index (range 1 _returnvalue_2)
        (Utilities|Array|SetArrayElem (Variables|Default|GetStored_MovementDirections) (- _index 1) (Utilities|Array|Get(acopy) (Variables|Default|GetStored_MovementDirections) _index)))
      (Utilities|Array|SetArrayElem (Variables|Default|GetStored_MovementDirections) _returnvalue_2 (LocalVariables|GetAddToStoredMovmentDirections))
      ;[1 1 1] Get Average Movement Direction and Store it to a variable
      (for _array_element (Variables|Default|GetStored_MovementDirections)
        (LocalVariables|SetTempAddedDirections (+ _array_element (LocalVariables|GetTempAddedDirections))))
      (Variables|Default|SetCurrent_MovementDirection (/ (LocalVariables|GetTempAddedDirections) (Math|Conversions|ToFloat(Integer) (Utilities|Array|Length (Variables|Default|GetStored_MovementDirections)))))
      (Variables|Default|SetHiltDirection (- (Variables|Default|GetCur_Loc) (Transformation|GetWorldLocation (Variables|Components|GetHiltFollower))))
      (return (Variables|Default|GetCurrent_MovementDirection))
      (else
        (Utilities|Array|Add (Variables|Default|GetStored_MovementDirections) _output_get)))))

(fn CalcDamageDirectionModifier
  (params (Hit%20Normald :type Vector))
  (for _array_element (Components|GetChildrenComponents (Variables|Default|GetDamage%20Direction%20Components) false)
    (bind _asarrow_component (Utilities|Casting|CastToArrowComponent _array_element)
      (:then
        ;[1 1 1] Store largest damage direction modifier value
        (LocalVariables|SetL_Stored%20Damage%20Direction%20Modifier (Math|Float|Max(Float) (Math|Curves|GetFloatValue (Variables|Setup|GetDamage%20Direction%20Modifier%20interp%20curve) (Math|Float|Clamp(Float) (* (Math|Vector|DotProduct (Math|Vector|Normalize (Math|Vector|GetForwardVector _asarrow_component)) (Math|Vector|Normalize Hit%20Normald)) -1.0))) (LocalVariables|GetL_Stored%20Damage%20Direction%20Modifier))))
      (:CastFailed
        (Development|PrintString (Utilities|String|Append (Utilities|GetDisplayName self) " contains a non arrow component inside of damage direction components.")))))
  (return (LocalVariables|GetL_Stored%20Damage%20Direction%20Modifier)))